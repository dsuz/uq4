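; BP_HUDIngame is the in-game HUD that shows a start screen and a running timer.
; On BeginPlay it creates the WBP_Timer and WBP_Start widgets for the owning player controller and adds both to the viewport.
; Each Tick it casts the game mode to ThirdPersonGameMode and pushes its elapsed seconds into the timer widget.
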(event `self.ReceiveBeginPlay`
  (bind _returnvalue (`self.GetOwningPlayerController`))
  (`|ExecutionSequence`
    (:`then_0`
      (bind _returnvalue_2 (`|CreateWidget` "/Game/WBP_Timer.WBP_Timer_C" _returnvalue))
      (bind _output_get (set `self.TimerWidget` _returnvalue_2))
      (`UserWidget.AddToViewport` _output_get 0))
    (:`then_1`
      (bind _returnvalue_3 (`|CreateWidget` "/Game/WBP_Start.WBP_Start_C" _returnvalue))
      (`UserWidget.AddToViewport` _returnvalue_3 0))))

(event `self.ReceiveTick`
  (params (DeltaSeconds :type "Float (single-precision)"))
  (bind _asthird_person_game_mode (cast `ThirdPersonGameMode` (`GameplayStatics.GetGameMode`)))
  (`/Game/WBP_Timer.UpdateTimer` (`self.TimerWidget`) (`ThirdPersonGameMode.GetElapsedSeconds` _asthird_person_game_mode)))

(fn `UserConstructionScript`)