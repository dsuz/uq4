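; BP_Goal is a goal actor that sets off a repeating Niagara fireworks (hanabi) effect when the player reaches it.
; On BeginPlay it caches the world locations of its scene components named with "HanabiSpawnPoint".
; The first overlap by BP_UQ4Player passes a DoOnce into PlayGoalEffect.
; That event spawns the effect at every cached location and re-calls itself through a short Delay, looping indefinitely.
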(event `self.ReceiveBeginPlay`
  (`self.Initialize`))

(event `self.ReceiveActorBeginOverlap`
  (params (OtherActor :type "Actor Object Reference"))
  (cast `/Game/UnrealQuest4_Game/ThirdPerson/Blueprints/BP_UQ4Player` OtherActor)
  (`/Engine/EditorBlueprintResources/StandardMacros.DoOnce` false
    (:`Completed`
      (`self.PlayGoalEffect`))))

(event `Initialize`
  (for _array_element (`self.K2_GetComponentsByClass` "/Script/Engine.SceneComponent")
    (if (`KismetStringLibrary.Contains` (`KismetSystemLibrary.GetObjectName` _array_element) "HanabiSpawnPoint")
      (`KismetArrayLibrary.Array_Add` (`self.HanabiSpawnLocations`) (`SceneComponent.K2_GetComponentLocation` _array_element)))))

(event `PlayGoalEffect`
  ;[1 1 1] エフェクトを表示する（ループ）
  (for _array_element (`self.HanabiSpawnLocations`)
    (`NiagaraFunctionLibrary.SpawnSystemAtLocation` (`self.NiagaraEffect`) _array_element)
    (`KismetSystemLibrary.Delay` 0.8)
    (`self.PlayGoalEffect`)))

(fn `UserConstructionScript`)